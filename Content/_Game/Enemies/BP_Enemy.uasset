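; BP_Enemy is the enemy Blueprint that handles its health bar widget and floating damage numbers.
; On BeginPlay it links the HealthBar component's WBP_EnemyHealthBar to itself and hides it, with show and hide events toggling visibility.
; Hit events spawn a WBP_HitNumber at the projected screen position of the hit, store it with its world location, and animate it with damage and headshot info.
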(event `self.ReceiveBeginPlay`
  (bind _aswbp_enemy_health_bar (cast `/Game/_Game/HUD/WBP_EnemyHealthBar` (`WidgetComponent.GetUserWidgetObject` (`self.HealthBar`))))
  (set `/Game/_Game/HUD/WBP_EnemyHealthBar.Enemy` self _aswbp_enemy_health_bar)
  (`Widget.SetVisibility` (`WidgetComponent.GetUserWidgetObject` (`self.HealthBar`)) "Hidden"))

(event `self.ShowHealthBar`
  (`Widget.SetVisibility` (`WidgetComponent.GetUserWidgetObject` (`self.HealthBar`)) "Visible")
  (`parent.ShowHealthBar`))

(event `self.HideHealthBar`
  (`Widget.SetVisibility` (`WidgetComponent.GetUserWidgetObject` (`self.HealthBar`)) "Hidden"))

(event `self.ShowHitNumber`
  (params (Damage :type Integer) (HitLocation :type "Vector Structure") (bHeadshot :type Boolean))
  (bind _returnvalue (`|CreateWidget` "/Game/_Game/HUD/WBP_HitNumber.WBP_HitNumber_C"))
  (`UserWidget.AddToViewport` _returnvalue 0)
  (`UserWidget.SetPositionInViewport` _returnvalue (`GameplayStatics.ProjectWorldToScreen` (`GameplayStatics.GetPlayerController` 0) HitLocation) true)
  (`self.StoreHitNumber` _returnvalue HitLocation)
  (set `/Game/_Game/HUD/WBP_HitNumber.HitText` (`KismetTextLibrary.Conv_IntToText` Damage) _returnvalue)
  (`UserWidget.PlayAnimationForward` _returnvalue (`/Game/_Game/HUD/WBP_HitNumber.HitNumberAnimation` _returnvalue) 1.0 false)
  (set `/Game/_Game/HUD/WBP_HitNumber.HeadShot` bHeadshot _returnvalue))

(fn `UserConstructionScript`)