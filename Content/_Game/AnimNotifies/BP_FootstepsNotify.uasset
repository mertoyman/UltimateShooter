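; BP_FootstepsNotify is an animation notify that produces surface-dependent footstep sounds and particles for BP_ShooterCharacter.
; It queries the character's physical surface and selects a matching sound, defaulting to wood, setting a Niagara effect only for stone, grass and water.
; The sound plays at the BoneName socket when ShouldPlaySound is set, while the effect spawn is called there regardless.
; Wood, metal and tile leave the effect variable unchanged.
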(fn `Received_Notify`
  (params (MeshComp :type "SkeletalMeshComponent Object Reference") (Animation :type "AnimSequenceBase Object Reference"))
  (returns (ReturnValue :type Boolean))
  (locals (FootstepSound :type "SoundCue Object Reference" :default "SoundCue'/Game/_Game/Assets/Sounds/Footsteps/Footstep_Wood.Footstep_Wood'") (FootstepNiagaraSystem :type "NiagaraSystem Object Reference" :default null))
  (bind _returnvalue (`SceneComponent.GetSocketLocation` MeshComp (`self.BoneName`)))
  (bind _asbp_shooter_character (cast `/Game/_Game/Character/BP_ShooterCharacter` (`ActorComponent.GetOwner` MeshComp)))
  (bind _returnvalue_2 (`ShooterCharacter.GetPhysicalSurface` _asbp_shooter_character))
  (switch `EPhysicalSurface` _returnvalue_2
    (:`SurfaceType_Default`
      (set `local.FootstepSound` "/Game/_Game/Assets/Sounds/Footsteps/Footstep_Wood.Footstep_Wood"))
    (:`SurfaceType1`
      (set `local.FootstepSound` "/Game/_Game/Assets/Sounds/Footsteps/Footstep_Metal.Footstep_Metal"))
    (:`SurfaceType2`
      (set `local.FootstepSound` "/Game/_Game/Assets/Sounds/Footsteps/Footstep_Stone.Footstep_Stone")
      (set `local.FootstepNiagaraSystem` "/Game/A_Surface_Footstep/Niagara_FX/ParticleSystems/PSN_Dirt_Surface.PSN_Dirt_Surface"))
    (:`SurfaceType3`
      (set `local.FootstepSound` "/Game/_Game/Assets/Sounds/Footsteps/Footstep_Tile.Footstep_Tile"))
    (:`SurfaceType4`
      (set `local.FootstepSound` "/Game/_Game/Assets/Sounds/Footsteps/Footstep_Grass.Footstep_Grass")
      (set `local.FootstepNiagaraSystem` "/Game/A_Surface_Footstep/Niagara_FX/ParticleSystems/PSN_Grass_Surface.PSN_Grass_Surface"))
    (:`SurfaceType5`
      (set `local.FootstepSound` "/Game/_Game/Assets/Sounds/Footsteps/Footstep_Water.Footstep_Water")
      (set `local.FootstepNiagaraSystem` "/Game/A_Surface_Footstep/Niagara_FX/ParticleSystems/PSN_WaterLight_Surface.PSN_WaterLight_Surface")))
  (if (`self.bShouldPlaySound`)
    (`GameplayStatics.PlaySoundAtLocation` (`local.FootstepSound`) _returnvalue (struct) 1.0 1.0 0.0 null null null))
  (`NiagaraFunctionLibrary.SpawnSystemAtLocation` (`local.FootstepNiagaraSystem`) _returnvalue)
  (return true))