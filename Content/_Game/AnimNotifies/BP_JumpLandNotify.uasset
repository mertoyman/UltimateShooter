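; Animation notify that plays a surface-specific landing sound when a shooter character lands from a jump.
; It casts the mesh owner to BP_ShooterCharacterBase and asks it for the physical surface underfoot.
; That surface selects a metal, stone, tile, grass or water sound, with concrete as the fallback, played at the character's location.
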(fn `Received_Notify`
  (params (MeshComp :type "SkeletalMeshComponent Object Reference") (Animation :type "AnimSequenceBase Object Reference"))
  (returns (ReturnValue :type Boolean))
  (locals (LandingSound :type "SoundCue Object Reference" :default "SoundCue'/Game/_Game/Assets/Sounds/Footsteps/Land_Stone.Land_Stone'"))
  (bind _returnvalue (`ActorComponent.GetOwner` MeshComp))
  (bind _asbp_belica_character (cast `/Game/_Game/Character/BP_ShooterCharacterBase` _returnvalue))
  (bind _returnvalue_2 (`ShooterCharacter.GetPhysicalSurface` _asbp_belica_character))
  (switch `EPhysicalSurface` _returnvalue_2
    (:`SurfaceType_Default`
      (set `local.LandingSound` "/Game/_Game/Assets/Sounds/Footsteps/Land_Concrete.Land_Concrete"))
    (:`SurfaceType1`
      (set `local.LandingSound` "/Game/_Game/Assets/Sounds/Footsteps/Land_Metal.Land_Metal"))
    (:`SurfaceType2`
      (set `local.LandingSound` "/Game/_Game/Assets/Sounds/Footsteps/Land_Stone.Land_Stone"))
    (:`SurfaceType3`
      (set `local.LandingSound` "/Game/_Game/Assets/Sounds/Footsteps/Land_Tile.Land_Tile"))
    (:`SurfaceType4`
      (set `local.LandingSound` "/Game/_Game/Assets/Sounds/Footsteps/Land_Grass.Land_Grass"))
    (:`SurfaceType5`
      (set `local.LandingSound` "/Game/_Game/Assets/Sounds/Footsteps/Land_Water.Land_Water")))
  (`GameplayStatics.PlaySoundAtLocation` (`local.LandingSound`) (`Actor.K2_GetActorLocation` _returnvalue) (struct) 1.0 1.0 0.0 null null null)
  (return true))