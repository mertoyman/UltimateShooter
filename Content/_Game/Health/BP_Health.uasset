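; BP_Health is a health pickup that heals shooter characters when they touch it.
; When an actor overlaps its Sphere, it casts to BP_ShooterCharacterBase and acts only if that character's Health is below MaxHealth.
; It adds HealingAmount to Health, capped at MaxHealth, then plays a pickup sound at its location and destroys itself.
; Characters at full health leave the pickup in place.
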(event `self.Sphere.OnComponentBeginOverlap`
  (params (OverlappedComponent :type "PrimitiveComponent Object Reference") (OtherActor :type "Actor Object Reference") (OtherComp :type "PrimitiveComponent Object Reference") (OtherBodyIndex :type Integer) (bFromSweep :type Boolean) (SweepResult :type "HitResult Structure (by ref)"))
  (bind _asbp_shooter_character_base (cast `/Game/_Game/Character/BP_ShooterCharacterBase` OtherActor))
  (bind _health (`ShooterCharacter.Health` _asbp_shooter_character_base))
  (bind _maxhealth (`ShooterCharacter.MaxHealth` _asbp_shooter_character_base))
  (if (< _health _maxhealth)
    (bind _returnvalue (+ _health (`self.HealingAmount`)))
    (if (> _returnvalue _maxhealth)
      (set `ShooterCharacter.Health` (`ShooterCharacter.MaxHealth` _asbp_shooter_character_base) _asbp_shooter_character_base)
      (else
        (set `ShooterCharacter.Health` _returnvalue _asbp_shooter_character_base)))
    (`GameplayStatics.PlaySoundAtLocation` (`self.HealingPickupSound`) (`self.K2_GetActorLocation`) (struct) 1.0 1.0 0.0 null null null)
    (`self.K2_DestroyActor`)))

(fn `UserConstructionScript`)